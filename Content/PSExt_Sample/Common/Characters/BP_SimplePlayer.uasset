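; Sample player Blueprint that displays its MetaCommId as a name tag on a Plane component.
; On BeginPlay it creates a dynamic M_PlayerName material and binds to the ID update dispatcher.
; Each update creates a small canvas render target, which draws the ID's first five characters as outlined text on a green fill.
; That render target feeds the material's Texture parameter on the Plane.
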(event `self.ReceiveBeginPlay`
  ;[1 1 1] MetaCommIdを描画するためのマテリアルを作成します。
  (bind _returnvalue (`PrimitiveComponent.CreateDynamicMaterialInstance` (`self.Plane`) 0 "/Game/PSExt_Sample/Common/Materials/M_PlayerName.M_PlayerName" "None"))
  (set `self.BillboardMaterial` _returnvalue)
  ;[1 1 1] MetaCommIdの更新があった場合に、ＩＤを書き換えます。
  (add `self.UpdateIdEventDispatcher` (delegate `カスタムイベント`)))

(event `カスタムイベント` :!signature `self.UpdateIdEventDispatcher`
  (params (PlayerId :type String) (MetaCommId :type String))
  (bind _billboardmaterial (`self.BillboardMaterial`))
  ;[1 1 1] MetaCommIdの更新があった場合に、ＩＤを書き換えます。
  (set `self.Meta Comm Id` MetaCommId)
  (bind _returnvalue (`CanvasRenderTarget2D.CreateCanvasRenderTarget2D` "/Script/Engine.CanvasRenderTarget2D" 100 40))
  (add `CanvasRenderTarget2D.OnCanvasRenderTargetUpdate` _returnvalue (delegate `CanvasRender`))
  (`CanvasRenderTarget2D.UpdateResource` _returnvalue)
  (`PrimitiveComponent.SetMaterial` (`self.Plane`) 0 _billboardmaterial)
  (`MaterialInstanceDynamic.SetTextureParameterValue` _billboardmaterial "Texture" _returnvalue))

(event `CanvasRender`
  (params (Canvas :type "Canvas Object Reference") (Width :type Integer) (Height :type Integer))
  ;[1 1 1] MetaCommIdの更新があった場合に、ＩＤを書き換えます。
  (`Canvas.K2_DrawTexture` Canvas null (0.0 0.0) (`KismetMathLibrary.MakeVector2D` (`KismetMathLibrary.Conv_IntToDouble` Width) (`KismetMathLibrary.Conv_IntToDouble` Height)) (0.0 0.0) (1.0 1.0) (struct :`G` 1.0 :`A` 1.0) "BLEND_Opaque" 0.0 (0.5 0.5))
  (`Canvas.K2_DrawText` Canvas "/Game/PSExt_Sample/Common/Materials/NameFont.NameFont" (`KismetStringLibrary.Left` (`self.Meta Comm Id`) 5) (10.0 0.0) (1.0 1.0) (`self.NameColor`) 0.0 (struct :`A` 1.0) (1.0 1.0) false false true (struct :`A` 1.0)))

(fn `UserConstructionScript`)