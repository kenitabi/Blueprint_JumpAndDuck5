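; Sample Pixel Streaming Ext player character that handles each streamed player's spawn, disconnect and input.
; Binds plugin delegates after a short delay, spawning or reusing an AI-controlled BP_ThirdPersonCharacter as target and matching BP_SceneCapture by SceneId for camera mode and yaw.
; Mouse and touch share one path: drags past a deadzone rotate the controller by viewport-relative swipe, while taps line-trace through the scene capture.
; DataChannel messages echo back; events print debug text.
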(event EventBeginPlay
  (|CallParentFunction)
  (CallFunction|PSExtEvent))

(event Custom|OnScreenTouched
  (params (Loaction :type Vector%202D%20Structure))
  (bind _current_scene_capture (Variables|Default|GetCurrent%20Scene%20Capture))
  ;[1 1 1] タッチ位置の当たり判定
  (Utilities|IsValid _current_scene_capture
    (:Is%20Valid
      (bind (_worldposition _worlddirection) (Class|SceneCaptureActorComponent|DeprojecttoWorld (Variables|/PixelStreamingExt/BP_SceneCapture.BP_SceneCapture_C|GetSceneCaptureActor _current_scene_capture) Loaction))
      (bind (_outhits _returnvalue) (Collision|MultiLineTraceByChannel _worldposition (+ _worldposition (* _worlddirection 10000)) "TraceTypeQuery3" false 0 "None"))
      (if _returnvalue
        (bind _array_element (Utilities|Array|ForEachLoopwithBreak _outhits)
          (:LoopBody
            (Development|PrintString (Utilities|GetDisplayName (.HitActor (Collision|BreakHitResult _array_element))))))
        (else
          (Development|PrintString "Not Hit"))))))

(event Custom|Touched
  (params (TocuhLocation :type Vector%202D%20Structure))
  ;[0 0 0] タッチ
  ;;[1 1 1] タッチ開始
  (Variables|TouchEvent|SetTouchStartLocation TocuhLocation)
  (Variables|TouchEvent|SetTouchStartRotation (Pawn|GetControlRotation :!class /Script/Engine.Pawn)))

(event Custom|TouchReleased
  ;[0 0 0] タッチ
  ;;[1 1 1] タッチ終了
  (if (Variables|TouchEvent|GetEnableCameraRotate)
    (Variables|TouchEvent|SetRotationInput "0, 0, 0")
    (Variables|TouchEvent|SetEnableCameraRotate false)
    (else
      (CallFunction|OnScreenTouched (Variables|TouchEvent|GetTouchStartLocation)))))

(event Custom|TouchMoved
  (params (TouchLocation :type Vector%202D%20Structure))
  (bind _touchstartlocation (Variables|TouchEvent|GetTouchStartLocation))
  (bind _returnvalue (- TouchLocation _touchstartlocation))
  ;[0 0 0] タッチ
  ;;[1 1 1] タッチ移動
  (if (Variables|TouchEvent|GetEnableCameraRotate)
    (CallFunction|RotateCamera (Math|Conversions|ToVector(Vector2D) _returnvalue) :!label _label)
    (elif (>= (Math|Vector2D|Vector2DLength _returnvalue) (Variables|TouchEvent|GetCameraDeadzone))
      (Variables|TouchEvent|SetEnableCameraRotate true)
      (goto _label))))

(event Custom|RotateCamera
  (params (MoveDelta :type Vector))
  ;[1 1 1] 回転処理
  (bind _returnvalue (CallFunction|CalculateRotationbyMoveDelta MoveDelta))
  (Pawn|SetControlRotation (Pawn|GetController) _returnvalue))

(event Custom|PSExtEvent
  (Utilities|FlowControl|Delay 0.2)
  (Utilities|FlowControl|Sequence
    (:then_0
      ;[1 1 1] JSONが送られてきた時の処理を行います。
      (EventDispatchers|BindEventtoOnRecievedJsonfromDataChennel (delegate Custom|OnRecievedJsonFromDataChannelEvent)))
    (:then_1
      ;[1 1 1] プレイヤーが接続してきた時の処理を行います。
      (EventDispatchers|BindEventtoOnSpawnPlayerCharacter (delegate Custom|OnSpawnPlayerCharacterEvent)))
    (:then_2
      ;[1 1 1] プレイヤーが切断した時の処理を行います。
      (EventDispatchers|BindEventtoOnDestroyPlayerCharacter (delegate Custom|OnDestroyPlayerCharacterEvent)))
    (:then_3
      ;[1 1 1] カメラ移動に失敗した時の処理を行います。
      (EventDispatchers|BindEventtoOnFailedtoSwitchCamera (delegate Custom|OnFailedToSwitchCameraEvent)))
    (:then_4
      ;[1 1 1] PlayerDelegate の取得
      (bind _asplayer_controller (Utilities|Casting|CastToPlayerController (Pawn|GetController)))
      (bind _returnvalue (Class|PixelStreamingExtBlueprints|GetPixelStreamingExtPlayerDelegates (Utilities|String|ToString(Integer) (Class|GameplayStatics|GetPlayerControllerID _asplayer_controller))))
      ;[1 1 1] マウス関連イベントの設定
      (EventDispatchers|AssignOnMouseUpEvent _returnvalue (delegate Custom|Player_OnMouseUpEvent))
      (EventDispatchers|AssignOnMouseDownEvent _returnvalue (delegate Custom|Player_OnMouseDownEvent))
      (EventDispatchers|AssignOnMouseMoveEvent _returnvalue (delegate Custom|Player_OnMouseMoveEvent))
      ;[1 1 1] タッチ関連イベントの設定
      (EventDispatchers|AssignOnTouchStartEvent _returnvalue (delegate Custom|Player_OnTouchStartEvent))
      (EventDispatchers|AssignOnTouchEndEvent _returnvalue (delegate Custom|Player_OnTouchEndEvent))
      (EventDispatchers|AssignOnTouchMoveEvent _returnvalue (delegate Custom|Player_OnTouchMoveEvent)))))

(event Custom|OnRecievedJsonFromDataChannelEvent
  (params (PlayerId :type String) (Descriptor :type String))
  ;[1 1 1] JSONが送られてきた時の処理を行います。
  (CallFunction|OnReceivedJsonfromDataChannel PlayerId Descriptor)
  (Development|PrintText (Utilities|Text|FormatText "@@@ On Received Json Event. PlayerId={0} Descriptor={1}" PlayerId Descriptor)))

(event Custom|OnSpawnPlayerCharacterEvent
  (params (PlayerId :type String) (MetaCommId :type String) (SceneId :type String))
  ;[1 1 1] プレイヤーが接続してきた時の処理を行います。
  (CallFunction|SpawnPlayerCharacter PlayerId MetaCommId SceneId)
  (Development|PrintText (Utilities|Text|FormatText "@@@ On Spawn Player Character Event. PlayerId={0} MetaCommId={1}" PlayerId MetaCommId)))

(event Custom|OnDestroyPlayerCharacterEvent
  (params (PlayerId :type String))
  ;[1 1 1] プレイヤーが切断した時の処理を行います。
  (CallFunction|DestroyPlayerCharacter PlayerId)
  (Development|PrintText (Utilities|Text|FormatText "@@@ On Destroy Player Character Event. PlayerId={0} " PlayerId)))

(event Custom|Player_OnMouseDownEvent
  (params (PlayerId :type String) (Button :type Integer) (ScreenLocation :type Vector%202D%20Structure))
  (bind (_x _y) (Math|Vector2D|BreakVector2D ScreenLocation))
  ;[1 1 1] マウス関連イベントの設定
  (CallFunction|Touched ScreenLocation)
  (Development|PrintText (Utilities|Text|FormatText "Player_OnMouseDownEvent PlayerId: {0}, Button: {1}, ScreenLocation: ({2}, {3})" PlayerId Button _x _y)))

(event Custom|Player_OnMouseMoveEvent
  (params (PlayerId :type String) (ScreenLocation :type Int%20Point%20Structure) (Delta :type Int%20Point%20Structure))
  (bind (_x _y) (Utilities|Struct|BreakIntPoint ScreenLocation))
  (bind (_x_2 _y_2) (Utilities|Struct|BreakIntPoint Delta))
  ;[1 1 1] マウス関連イベントの設定
  (CallFunction|TouchMoved (Math|Conversions|ToVector2D(IntPoint) ScreenLocation))
  (Development|PrintText (Utilities|Text|FormatText "Player_OnMouseMoveEvent PlayerId: {0},ScreenLocation: ({1}, {2}), Delta: ({3}, {4})" PlayerId _x _y _x_2 _y_2) false false) ; Moveでは大量のログが発生するため、通常はログ出力を抑止しています。
)

(event Custom|OnFailedToSwitchCameraEvent
  (params (PlayerId :type String) (SceneId :type String))
  ;[1 1 1] カメラ移動に失敗した時の処理を行います。
  (CallFunction|OnFailedtoSwitchCamera SceneId)
  (Development|PrintText (Utilities|Text|FormatText "@@@ On Failed to Switch Camera. SceneId={0} " SceneId))
  (Development|PrintText (Utilities|Text|ToText(String) (Variables|Default|GetPlayerId)) true true "(R=0.301284,G=0.150036,B=1.000000,A=1.000000)" 1e+01))

(event Custom|Player_OnMouseUpEvent
  (params (PlayerId :type String) (Button :type Integer) (ScreenLocation :type Vector%202D%20Structure))
  (bind (_x _y) (Math|Vector2D|BreakVector2D ScreenLocation))
  ;[1 1 1] マウス関連イベントの設定
  (CallFunction|TouchReleased)
  (Development|PrintText (Utilities|Text|FormatText "Player_OnMouseUpEvent PlayerId: {0}, Button: {1}, ScreenLocation: ({2}, {3})" PlayerId Button _x _y)))

(event Custom|Player_OnTouchStartEvent
  (params (PlayerId :type String) (TouchLocation :type Vector%202D%20Structure) (TouchForce :type Integer) (TouchIndex :type Integer))
  (bind (_x _y) (Math|Vector2D|BreakVector2D TouchLocation))
  ;[1 1 1] タッチ関連イベントの設定
  (CallFunction|Touched TouchLocation)
  (Development|PrintText (Utilities|Text|FormatText "Player_OnTouchStartEvent PlayerId: {0},TouchLocation: ({1}, {2}), TouchForce: {3}, TouchIndex: {4}" PlayerId _x _y TouchForce TouchIndex)))

(event Custom|Player_OnTouchEndEvent
  (params (PlayerId :type String) (TouchLocation :type Vector%202D%20Structure) (TouchForce :type Integer) (TouchIndex :type Integer))
  (bind (_x _y) (Math|Vector2D|BreakVector2D TouchLocation))
  ;[1 1 1] タッチ関連イベントの設定
  (CallFunction|TouchReleased)
  (Development|PrintText (Utilities|Text|FormatText "Player_OnTouchEndEvent PlayerId: {0},TouchLocation: ({1}, {2}), TouchForce: {3}, TouchIndex: {4}" PlayerId _x _y TouchForce TouchIndex)))

(event Custom|Player_OnTouchMoveEvent
  (params (PlayerId :type String) (TouchLocation :type Vector%202D%20Structure) (TouchForce :type Integer) (TouchIndex :type Integer))
  (bind (_x _y) (Math|Vector2D|BreakVector2D TouchLocation))
  ;[1 1 1] タッチ関連イベントの設定
  (CallFunction|TouchMoved TouchLocation)
  (Development|PrintText (Utilities|Text|FormatText "Player_OnTouchMoveEvent PlayerId: {0},TouchLocation: ({1}, {2}), TouchForce: {3}, TouchIndex: {4}" PlayerId _x _y TouchForce TouchIndex) false false) ; Moveでは大量のログが発生するため、通常はログ出力を抑止しています。
)

(fn ConstructionScript)

(fn SpawnPlayerCharacter
  (params (PlayerId :type String) (MetaCommId :type String) (SceneId :type String))
  (bind _cameramode (CallFunction|GetCameraModefromSceneId SceneId))
  (Variables|Default|SetCameraMode _cameramode)
  (bind (_result _character) (Default|FindPlayerCharacterbyMetaCommId (Variables|Default|GetCharacterManager) MetaCommId))
  (if _result
    ;[1 1 1] 既にキャラクターが存在する場合は、そのキャラクターをターゲットとして扱う。
    (CallFunction|AddCharacterandSetTargetCharacter PlayerId MetaCommId _character)
    (CallFunction|CallSimplePlayerEvent _character PlayerId MetaCommId)
    (CallFunction|SetControllerRotationbySceneId SceneId)
    (Default|InitScreenRes (Variables|Default|GetCurrent%20Scene%20Capture))
    (return)
    (else
      (bind _transform (CallFunction|GetFirstLocation SceneId))
      (Transformation|SetActorTransform _transform false true) ; 操作するキャラクターの位置に移動します。
      (bind _returnvalue (Game|SpawnActorfromClass "/Game/ThirdPerson/Blueprints/BP_ThirdPersonCharacter.BP_ThirdPersonCharacter_C" _transform "AdjustIfPossibleButAlwaysSpawn" "MultiplyWithRoot" 0 0))
      (Pawn|SpawnDefaultController _returnvalue) ; キャラクターにはAIController を設定しておきます。
      (CallFunction|AddCharacterandSetTargetCharacter PlayerId MetaCommId _returnvalue) ; 操作するキャラクターを Target Character に設定します。
      (CallFunction|CallSimplePlayerEvent _returnvalue PlayerId MetaCommId)
      (CallFunction|SetControllerRotationbySceneId SceneId)
      (Default|InitScreenRes (Variables|Default|GetCurrent%20Scene%20Capture))
      (return))))

(fn DestroyPlayerCharacter
  (params (PlayerId :type String))
  (bind _targetcharacter (Variables|Default|GetTargetCharacter))
  (Utilities|IsValid _targetcharacter
    (:Is%20Valid
      (Actor|DestroyActor _targetcharacter)
      (CallFunction|RemoveCharacterandClearTragetCharacter)
      (Default|InitScreenRes (Variables|Default|GetCurrent%20Scene%20Capture))
      (return))))

(fn OnReceivedJsonfromDataChannel
  (params (PlayerId :type String) (Descriptor :type String))
  (Development|PrintString Descriptor)
  (Class|PixelStreamingExtBlueprints|PixelStreamingExtSendCustomMessage PlayerId Descriptor) ; 送られてきたメッセージを送り返します。
)

(fn OnFailedtoSwitchCamera
  (params (SceneId :type String)))

(fn CallSimplePlayerEvent
  (params (Character :type Character%20Object%20Reference) (PlayerId :type String) (MetaCommId :type String))
  (bind _asbp_third_person_character (Utilities|Casting|CastToBP_ThirdPersonCharacter Character))
  (Default|CallUpdateIdEventDispatcher _asbp_third_person_character PlayerId MetaCommId))

(fn GetFirstLocation
  (params (SceneId :type String))
  (bind _firstlocationmap (Variables|Default|GetFirstLocationMap))
  (bind (_value _returnvalue) (Utilities|Map|Find _firstlocationmap SceneId))
  (if _returnvalue
    (return (Math|Conversions|ToTransform(Vector) _value))
    (else
      (return (Math|Transform|MakeTransform "0.000000,0.000000,500.000000")))))

(fn FindSceneCapturebySceneId
  (params (SceneId :type String))
  (bind _outactors (Actor|GetAllActorsOfClass "/PixelStreamingExt/BP_SceneCapture.BP_SceneCapture_C"))
  (for _array_element _outactors
    (if (Utilities|Enum|Equal(Enum) (Variables|/PixelStreamingExt/BP_SceneCapture.BP_SceneCapture_C|GetSceneId _array_element) SceneId)
      (return true _array_element)))
  (return false 0))

(fn SetControllerRotationbySceneId
  (params (SceneId :type String))
  (bind (_result _scenecapture) (CallFunction|FindSceneCapturebySceneId SceneId))
  (Variables|Default|SetCurrent%20Scene%20Capture _scenecapture)
  (if _result
    (Pawn|SetControlRotation (Pawn|GetController) (Math|Rotator|MakeRotator 0.0 0.0 (.yaw (Transformation|GetActorRotation _scenecapture)))) ; カメラの向きに合わせてコントローラーの回転を設定します。
  )
  (return))

(fn GetCameraModefromSceneId
  (params (SceneId :type String))
  (bind _outactors (Actor|GetAllActorsOfClass "/PixelStreamingExt/BP_SceneCapture.BP_SceneCapture_C"))
  (for _array_element _outactors
    (if (Utilities|Enum|Equal(Enum) (Variables|/PixelStreamingExt/BP_SceneCapture.BP_SceneCapture_C|GetSceneId _array_element) SceneId)
      (return (Variables|/PixelStreamingExt/BP_SceneCapture.BP_SceneCapture_C|GetCameraMode _array_element))))
  (return "ThirdPerson"))

(fn CalculateRotationbyMoveDelta
  (params (InVec :type Vector))
  (bind (_x _y) (Math|Vector|BreakVector InVec))
  (bind _touchstartrotation (Variables|TouchEvent|GetTouchStartRotation))
  (bind _current_scene_capture (Variables|Default|GetCurrent%20Scene%20Capture))
  (LocalVariables|SetCurrentForwardVector (Math|Vector|GetForwardVector _touchstartrotation))
  (LocalVariables|SetCalculatedYaw (.yaw (Math|Conversions|RotationFromXVector (Math|Vector|RotateVectorAroundAxis (LocalVariables|GetCurrentForwardVector) (|(((DeltaX*Sensitivity)*360)/ViewportX) _x (Variables|TouchEvent|GetCameraSensitivity) (Math|Conversions|ToFloat(Integer) (Variables|/PixelStreamingExt/BP_SceneCapture.BP_SceneCapture_C|GetWidth _current_scene_capture))) "0.000000,0.000000,1.000000"))))
  (LocalVariables|SetCalculatedPitch (.pitch (Math|Conversions|RotationFromXVector (Math|Vector|RotateVectorAroundAxis (LocalVariables|GetCurrentForwardVector) (|(((DeltaY*Sensitivity)*90)/ViewportY) _y (Variables|TouchEvent|GetCameraSensitivity) (Math|Conversions|ToFloat(Integer) (Variables|/PixelStreamingExt/BP_SceneCapture.BP_SceneCapture_C|GetHeight _current_scene_capture))) (Math|Vector|GetRightVector _touchstartrotation)))))
  (return (Math|Rotator|MakeRotator 0.0 (LocalVariables|GetCalculatedPitch) (LocalVariables|GetCalculatedYaw))))