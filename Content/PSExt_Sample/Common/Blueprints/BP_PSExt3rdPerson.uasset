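; Third-person multi-user manager for the PixelStreamingExt sample, linking plugin player and input events to per-player characters.
; InitPlayerControllers pre-creates a controller per scene ID and connects its scene-capture character to the signalling server.
; Camera select and going-away events reuse these pawns, toggling controller tick and MetaCommId instead of spawning, while connect and going-away start and stop streaming.
; JSON input is forwarded to the matching character; camera-switch handlers are effectively no-ops.
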(event `self.ReceiveBeginPlay`
  (`self.PixelStreamingExtEvent`) ; PixelStreaming拡張プラグインのイベントを登録します。
)

(event `PixelStreamingExtEvent`
  (`|ExecutionSequence`
    (:`then_0`
      (bind _returnvalue (`PixelStreamingExtBlueprints.GetPixelStreamingExtDelegates`))
      (add `PixelStreamingExtDelegates.OnCameraSwitchPrepareResponse` _returnvalue (delegate `OnCameraSwitchPrepareResponse`))
      (add `PixelStreamingExtDelegates.OnCameraSwitchResponse` _returnvalue (delegate `OnCameraSwitchResponse`))
      (add `PixelStreamingExtDelegates.OnCameraSwitchCancelResponse` _returnvalue (delegate `OnCameraSwitchCancel`))
      (add `PixelStreamingExtDelegates.OnCameraSelectRequest` _returnvalue (delegate `OnCameraSelectRequest`)))
    (:`then_1`
      (bind _returnvalue_2 (`PixelStreamingExtBlueprints.GetPixelStreamingExtDelegates`))
      (add `PixelStreamingExtDelegates.OnPlayerConnected` _returnvalue_2 (delegate `OnPlayerConnected`))
      (add `PixelStreamingExtDelegates.OnPlayerDisconnected` _returnvalue_2 (delegate `OnPlayerDisconnected`))
      (add `PixelStreamingExtDelegates.OnPlayerGoingAway` _returnvalue_2 (delegate `OnPlayerGoingAway`)))
    (:`then_2`
      (bind _returnvalue_3 (`AddComponent|NODE_AddPixelStreamingExtInput-1`))
      (add `PixelStreamingExtInput.OnInputEvent` _returnvalue_3 (delegate `OnInputEvent`))
      (`KismetSystemLibrary.PrintString` "Bind to PixelStreamingInput"))))

(event `OnCameraSelectRequest`
  (params (PlayerId :type String) (MetaCommId :type String) (SceneId :type String))
  (`self.Spawn Player Character` PlayerId MetaCommId SceneId)
  (`KismetSystemLibrary.PrintText` (`|FormatText` "@@ OnCameraSelectRequest  : result PlayerId={0}  MetaCommId={1}  SceneId={2}" PlayerId MetaCommId SceneId)))

(event `OnCameraSwitchPrepareResponse`
  (params (PlayerId :type String) (SceneId :type String) (Result :type Boolean))
  (`self.Process Camera Switch Prepare Response` PlayerId SceneId Result)
  (`KismetSystemLibrary.PrintText` (`|FormatText` "@@ OnCameraSwitchPrepareResponse: result={0}  PlayerId={1}  SceneId={2}" Result PlayerId SceneId)))

(event `OnCameraSwitchCancel`
  (params (PlayerId :type String) (SceneId :type String) (Result :type Boolean))
  (`KismetSystemLibrary.PrintText` (`|FormatText` "@@ OnCameraSwitchCancelResponse: result={0}  PlayreId={1}  SceneId={2}" Result PlayerId SceneId)))

(event `OnCameraSwitchResponse`
  (params (PlayerId :type String) (SceneId :type String) (Result :type Boolean))
  (`self.Process Camera Switch Response` PlayerId SceneId Result)
  (`KismetSystemLibrary.PrintText` (`|FormatText` "@@ OnCameraSwitchResponse: result={0}  PlayerId={1}  SceneId={2}" Result PlayerId SceneId)))

(event `OnPlayerGoingAway`
  (params (PlayerId :type String) (MetaCommId :type String))
  (`self.Despawn Player Character` PlayerId MetaCommId)
  (`self.Process Player Going Away` PlayerId MetaCommId)
  (`KismetSystemLibrary.PrintText` (`|FormatText` "@@ OnPlayerGoingAway PlayerId={0} MetaCommId={1}" PlayerId MetaCommId)))

(event `OnPlayerConnected`
  (params (PlayerId :type String))
  (`self.Process Player Connected` PlayerId)
  (`KismetSystemLibrary.PrintText` (`|FormatText` "@@ OnPlayerConnected PlayerId={0}" PlayerId)))

(event `OnPlayerDisconnected`
  (params (PlayerId :type String) (MetaCommId :type String))
  (`KismetSystemLibrary.PrintText` (`|FormatText` "@@ PlayerDisconnected PlayerId={0} MetaCommId={1}" PlayerId MetaCommId)))

(event `OnInputEvent`
  (params (PlayerId :type String) (Descriptor :type String))
  (`self.Process Recevied Json Event` PlayerId Descriptor)
  (`KismetSystemLibrary.PrintText` (`|FormatText` "@@ On Input Event PlayerId={0} Descriptor={1}" PlayerId Descriptor)))

(fn `Create Player Controller for Third Person`
  (params (PlayerId :type String) (SceneId :type String))
  (bind (_result _controller) (`/Game/PSExt_Sample/Common/Blueprints/BP_PSExtPlayerManager.Create Player Controller` (`self.BP_PSExtPlayerManager`) PlayerId "ThirdPerson" (`self.BP_PSExtCharacterManager`)))
  (if _result
    ;[1 1 1] 先にシグナリングサーバへの接続処理を行います。
    (bind _asbp_player_character_base (cast `/Game/PSExt_Sample/Common/Characters/BP_PlayerCharacterBase` (`Controller.K2_GetPawn` _controller)))
    (bind _asbp_scene_capture (cast `/PixelStreamingExt/BP_SceneCapture` (`ChildActorComponent.ChildActor` (`/Game/PSExt_Sample/Common/Characters/BP_PlayerCharacterBase.BP_SceneCapture` _asbp_player_character_base))))
    (`/PixelStreamingExt/BP_SceneCapture.Get ScenecaptureRes From Command Line` _asbp_scene_capture)
    (`/Game/PSExt_Sample/Common/Characters/BP_PlayerCharacterBase.ConnectToSignallingServer` _asbp_player_character_base (`local.SceneId`) (`local.PlayerId`)) ; SceneId と PlayerId の紐づけを行うために、引数に渡しています。
    (return)))

(fn `Despawn Player Character`
  (params (PlayerId :type String) (MetaCommId :type String))
  (bind (_result _character _controller) (`/Game/PSExt_Sample/Common/Blueprints/BP_PSExtPlayerManager.Find Player Character Base By PlayerId` (`self.BP_PSExtPlayerManager`) PlayerId))
  (if _result
    (`self.SetActorTickEnabled` _controller false) ; 未使用のControllerのTickをOff
    (`self.OnDestroyPlayerCharacter` _character (`local.PlayerId`))
    (`/Game/PSExt_Sample/Common/Characters/BP_PlayerCharacterBase.OnDestroyPlayerCharacter` _character (`local.PlayerId`))
    (set `/Game/PSExt_Sample/Common/Characters/BP_PlayerCharacterBase.MetaCommId` "" _character) ; Meta Comm Id に空文字を入れておく
    (return)
    (else
      (`KismetSystemLibrary.PrintText` (`|FormatText` "@@@ Character no longer exists. PlayerId={0} " (`local.PlayerId`))))))

(fn `Init Player Controllers`
  (params (SceneIds :type "Array of String"))
  (for (_array_element _array_index) SceneIds
    (`self.Create Player Controller for Third Person` (`KismetStringLibrary.Conv_IntToString` _array_index) _array_element))
  (`KismetSystemLibrary.PrintString` "All PlayerControllers creation is complete."))

(fn `Process Camera Switch Prepare Response`
  (params (PlayerId :type String) (SceneId :type String) (Result :type Boolean))
  (if (not Result)
    (`self.Process Failed To Switch Camera` PlayerId SceneId))
  (return))

(fn `Process Camera Switch Response`
  (params (PlayerId :type String) (SceneId :type String) (Result :type Boolean))
  (if (not Result)
    (`self.Process Failed To Switch Camera` PlayerId SceneId))
  (return))

(fn `Process Failed To Switch Camera`
  (params (PlayerId :type String) (SceneId :type String))
  (return))

(fn `Process Player Connected`
  (params (PlayerId :type String))
  (bind (_result _character) (`/Game/PSExt_Sample/Common/Blueprints/BP_PSExtPlayerManager.Find Player Character Base By PlayerId` (`self.BP_PSExtPlayerManager`) PlayerId))
  (if _result
    (`/Game/PSExt_Sample/Common/Characters/BP_PlayerCharacterBase.Start Streaming` _character) ; OnPlayerConnected が呼び出されたので、映像配信を開始します。
    (return)))

(fn `Process Player Going Away`
  (params (PlayerId :type String) (MetaCommId :type String))
  (bind (_result _character) (`/Game/PSExt_Sample/Common/Blueprints/BP_PSExtPlayerManager.Find Player Character Base By PlayerId` (`self.BP_PSExtPlayerManager`) PlayerId))
  (if _result
    (`/Game/PSExt_Sample/Common/Characters/BP_PlayerCharacterBase.Stop Streaming` _character)
    (return)))

(fn `Process Recevied Json Event`
  (params (PlayerId :type String) (Descriptor :type String))
  (bind (_result _character) (`/Game/PSExt_Sample/Common/Blueprints/BP_PSExtPlayerManager.Find Player Character Base By PlayerId` (`self.BP_PSExtPlayerManager`) PlayerId))
  (if _result
    (`self.OnRecievedJsonFromDataChennel` _character (`local.PlayerId`) (`local.Descriptor`))
    (`/Game/PSExt_Sample/Common/Characters/BP_PlayerCharacterBase.OnRecievedJsonFromDataChennel` _character (`local.PlayerId`) (`local.Descriptor`))
    (return)))

(fn `Spawn Player Character`
  (params (PlayerId :type String) (MetaCommId :type String) (SceneId :type String))
  (bind _result (`/Game/PSExt_Sample/Common/Blueprints/BP_PSExtPlayerManager.Is Exist Player Controller` (`self.BP_PSExtPlayerManager`) PlayerId)) ; PlayerId に紐づく Player Controller が存在する確認します。
  (if _result
    (bind (_result_2 _character _controller) (`/Game/PSExt_Sample/Common/Blueprints/BP_PSExtPlayerManager.Find Player Character Base By PlayerId` (`self.BP_PSExtPlayerManager`) PlayerId))
    (if _result_2
      (`self.SetActorTickEnabled` _controller true)
      (set `/Game/PSExt_Sample/Common/Characters/BP_PlayerCharacterBase.MetaCommId` (`local.MetaCommId`) _character)
      (`self.OnSpawnPlayerCharacter` _character (`local.PlayerId`) (`local.MetaCommId`) (`local.SceneId`))
      (`/Game/PSExt_Sample/Common/Characters/BP_PlayerCharacterBase.OnSpawnPlayerCharacter` _character (`local.PlayerId`) (`local.MetaCommId`) (`local.SceneId`))
      (return))
    (else
      (`KismetSystemLibrary.PrintText` (`|FormatText` "@@@ Not Found a PlayerController. PlayerId={0} MetaCommId={1}" (`local.PlayerId`) (`local.MetaCommId`)))
      (return))))

(fn `UserConstructionScript`)