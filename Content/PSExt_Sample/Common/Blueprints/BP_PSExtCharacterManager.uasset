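; BP_PSExtCharacterManager keeps track of player characters in the PSExt sample, keyed by MetaCommId.
; Add, remove and find functions wrap the CharactersMaps map that holds this registry.
; A separate helper reuses or adds a BP_PlayerCommon component on a given character, then sets its IDs, NPC flag and camera mode.
; A debug function prints every registered MetaCommId.
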(fn `Add Player Character`
  (params (MetaCommId :type String) (Character :type "Character Object Reference"))
  (`BlueprintMapLibrary.Map_Add` (`self.CharactersMaps`) MetaCommId Character)
  (return))

(fn `Add Player Common to Character`
  (params (Character :type "Character Object Reference") (PlayerId :type String) (MetaCommId :type String) (IsNPC :type Boolean) (CameraMode :type "PSExtCameraMode Enum" :default "Fixed"))
  (bind _returnvalue (`Actor.GetComponentByClass` Character "/Game/PSExt_Sample/Common/Blueprints/BP_PlayerCommon.BP_PlayerCommon_C"))
  (`/Engine/EditorBlueprintResources/StandardMacros.IsValid` _returnvalue
    (:`Is Valid`
      (`/Game/PSExt_Sample/Common/Blueprints/BP_PlayerCommon.Set Params` _returnvalue (`local.PlayerId`) (`local.MetaCommId`) (`local.IsNPC`) (`local.CameraMode`)) ; BP_PlayerCommonが存在する場合は、設定を変更のみ行います。
      (return))
    (:`Is Not Valid`
      (bind _returnvalue_2 (`|AddComponentByClass` Character "/Game/PSExt_Sample/Common/Blueprints/BP_PlayerCommon.BP_PlayerCommon_C")) ; キャラクターに BP_PlayerCommon が存在しない場合は追加します。
      (`/Game/PSExt_Sample/Common/Blueprints/BP_PlayerCommon.Set Params` _returnvalue_2 (`local.PlayerId`) (`local.MetaCommId`) (`local.IsNPC`) (`local.CameraMode`))
      (return))))

(fn `Find Player Character By MetaCommId`
  (params (MetaCommId :type String))
  (returns (Result :type Boolean) (Character :type "Character Object Reference"))
  (bind (_value _returnvalue) (`BlueprintMapLibrary.Map_Find` (`self.CharactersMaps`) MetaCommId))
  (return _returnvalue _value))

(fn `Remove Player Character`
  (params (MetaCommId :type String))
  (returns (Result :type Boolean))
  (bind _returnvalue (`BlueprintMapLibrary.Map_Remove` (`self.CharactersMaps`) MetaCommId))
  (return _returnvalue))

(fn `ShowPlayerCharacterDebugInfo`
  (bind _keys (`BlueprintMapLibrary.Map_Keys` (`self.CharactersMaps`)))
  (`KismetSystemLibrary.PrintString` "-----------------------")
  (for _array_element _keys
    (`KismetSystemLibrary.PrintString` _array_element))
  (`KismetSystemLibrary.PrintString` "===================="))