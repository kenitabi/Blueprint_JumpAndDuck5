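; BP_PSExtPlayerManager creates, finds and removes local player controllers for the PSExt sample, using PlayerId as the controller ID.
; Creation reuses an existing controller or spawns a local player, disables the controller's tick, then passes ID, camera mode and character manager to its BP_PlayerCharacterBase pawn.
; Successfully initialized controllers are recorded in a map, and removal also destroys the pawn.
; A helper approximates camera visibility with a forward-vector dot product against a threshold.
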(fn `Create Player Controller`
  (params (PlayerId :type String) (CameraMode :type "PSExtCameraMode Enum" :default "ThirdPerson") (CharacterManager :type "/Game/PSExt_Sample/Common/Blueprints/BP_PSExtCharacterManager Object Reference"))
  (returns (Result :type Boolean) (Controller :type "PlayerController Object Reference"))
  (bind _returnvalue (`GameplayStatics.GetPlayerControllerFromID` (`KismetStringLibrary.Conv_StringToInt` PlayerId)))
  (`KismetSystemLibrary.PrintString` (`KismetStringLibrary.Concat_StrStr` "Create Player Controller. PlayerId=" PlayerId))
  (`/Engine/EditorBlueprintResources/StandardMacros.IsValid` _returnvalue
    (:`Is Valid`
      ;[1 1 1] 既にPlayerControllerが存在している場合には初期化のみ行います。
      (`Actor.SetActorTickEnabled` _returnvalue false) ; 未使用のControllerのTickをOff
      (bind _result (`self.Init Player Character Base` _returnvalue (`Controller.K2_GetPawn` _returnvalue) (`local.PlayerId`) (`local.CameraMode`) (`local.CharacterManager`)))
      (return _result _returnvalue))
    (:`Is Not Valid`
      ;[1 1 1] PlayerController が存在しない場合には作成し、初期化を行います。
      (bind _returnvalue_2 (`GameplayStatics.CreatePlayer` (`KismetStringLibrary.Conv_StringToInt` PlayerId)))
      (`Actor.SetActorTickEnabled` _returnvalue_2 false) ; 未使用のControllerのTickをOff
      (bind _result_2 (`self.Init Player Character Base` _returnvalue_2 (`Controller.K2_GetPawn` _returnvalue_2) (`local.PlayerId`) (`local.CameraMode`) (`local.CharacterManager`)))
      (return _result_2 _returnvalue_2))))

(fn `Destroy Player Controller`
  (params (PlayerId :type String))
  (bind _returnvalue (`GameplayStatics.GetPlayerControllerFromID` (`KismetStringLibrary.Conv_StringToInt` PlayerId)))
  (`BlueprintMapLibrary.Map_Remove` (`self.PlayerControllerMaps`) PlayerId)
  (`/Engine/EditorBlueprintResources/StandardMacros.IsValid` _returnvalue
    (:`Is Valid`
      (`GameplayStatics.RemovePlayer` _returnvalue true)
      (return))
    (:`Is Not Valid`
      (return))))

(fn `Find Player Character Base By PlayerId`
  (params (PlayerId :type String))
  (returns (Result :type Boolean) (Character :type "/Game/PSExt_Sample/Common/Characters/BP_PlayerCharacterBase Object Reference") (Controller :type "PlayerController Object Reference"))
  (locals (PlayerController :type "PlayerController Object Reference"))
  (bind _returnvalue (`GameplayStatics.GetPlayerControllerFromID` (`KismetStringLibrary.Conv_StringToInt` PlayerId)))
  (`/Engine/EditorBlueprintResources/StandardMacros.IsValid` _returnvalue
    (:`Is Valid`
      (set `local.PlayerController` _returnvalue)
      (bind _asbp_player_character_base (cast `/Game/PSExt_Sample/Common/Characters/BP_PlayerCharacterBase` (`Controller.K2_GetPawn` (`local.PlayerController`)))
        (:`then`
          (return true _asbp_player_character_base (`local.PlayerController`)))
        (:`CastFailed`
          (return false null null))))
    (:`Is Not Valid`
      (`KismetSystemLibrary.PrintText` (`|FormatText` "Not found player controller: {0}" PlayerId)))))

(fn `Init Player Character Base`
  (params (Controller :type "PlayerController Object Reference") (Pawn :type "Pawn Object Reference") (PlayerId :type String) (CameraMode :type "PSExtCameraMode Enum" :default "ThirdPerson") (CharacterManager :type "/Game/PSExt_Sample/Common/Blueprints/BP_PSExtCharacterManager Object Reference"))
  (returns (Result :type Boolean))
  (bind _asbp_player_character_base (cast `/Game/PSExt_Sample/Common/Characters/BP_PlayerCharacterBase` Pawn)
    (:`then`
      (set `/Game/PSExt_Sample/Common/Characters/BP_PlayerCharacterBase.PlayerId` PlayerId _asbp_player_character_base)
      (set `/Game/PSExt_Sample/Common/Characters/BP_PlayerCharacterBase.CameraMode` CameraMode _asbp_player_character_base)
      (set `/Game/PSExt_Sample/Common/Characters/BP_PlayerCharacterBase.CharacterManager` CharacterManager _asbp_player_character_base)
      (`BlueprintMapLibrary.Map_Add` (`self.PlayerControllerMaps`) PlayerId Controller)
      (return true))
    (:`CastFailed`
      (return false))))

(fn `Is Exist Player Controller`
  (params (PlayerId :type String))
  (returns (Result :type Boolean))
  (`/Engine/EditorBlueprintResources/StandardMacros.IsValid` (`GameplayStatics.GetPlayerControllerFromID` (`KismetStringLibrary.Conv_StringToInt` PlayerId))
    (:`Is Valid`
      (return true))
    (:`Is Not Valid`
      (return false))))

(fn `Is In Camera`
  (params (Character :type "Character Object Reference") (Camera :type "/PixelStreamingExt/BP_SceneCapture Object Reference") (Offset :type "Float (double-precision)"))
  (returns (Result :type Boolean))
  (return (> (`KismetMathLibrary.Dot_VectorVector` (`Actor.GetActorForwardVector` Camera) (`KismetMathLibrary.Normal` (- (`Actor.K2_GetActorLocation` Character) (`Actor.K2_GetActorLocation` Camera)))) Offset)))