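; BP_Barrier is an obstacle actor with a configurable mesh, set in the construction script, and a spinning coin.
; Hitting its box calls HitMessage on the other actor, passes the arrow's transform to the game mode and plays a bomb sound once.
; A separate sound trigger plays a cheer once when the player overlaps it.
; The coin spawns a burst effect whenever the third-person character overlaps it, without being removed.
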(event `self.ReceiveTick`
  (params (DeltaSeconds :type "Float (single-precision)"))
  ;[1 1 1] コイン回転
  (`SceneComponent.K2_AddLocalRotation` (`self.SM_Coin`) (struct :`Yaw` 5.0) false false))

(event `self.Box.OnComponentHit`
  (params (HitComponent :type "PrimitiveComponent Object Reference") (OtherActor :type "Actor Object Reference") (OtherComp :type "PrimitiveComponent Object Reference") (NormalImpulse :type "Vector Structure") (Hit :type "HitResult Structure (by ref)"))
  (message `/Game/01_Spline/BPI_Player.Hit` OtherActor)
  (message `/Game/01_Spline/BPI_Player.NotifyToGM` (`GameplayStatics.GetGameMode`) (`SceneComponent.K2_GetComponentToWorld` (`self.Arrow`)))
  (`/Engine/EditorBlueprintResources/StandardMacros.DoOnce` false
    (:`Completed`
      (`GameplayStatics.PlaySoundAtLocation` "/Game/Audio/BombPower_Full.BombPower_Full" (`self.K2_GetActorLocation`) (struct) 1.0 1.0 0.0 null null null null))))

(event `self.SoumdCollision.OnComponentBeginOverlap`
  (params (OverlappedComponent :type "PrimitiveComponent Object Reference") (OtherActor :type "Actor Object Reference") (OtherComp :type "PrimitiveComponent Object Reference") (OtherBodyIndex :type Integer) (bFromSweep :type Boolean) (SweepResult :type "HitResult Structure (by ref)"))
  (if (== OtherActor (`GameplayStatics.GetPlayerCharacter` 0))
    (`/Engine/EditorBlueprintResources/StandardMacros.DoOnce` false
      (:`Completed`
        (`GameplayStatics.PlaySoundAtLocation` "/Game/Audio/Knight_Cheers/Yay_Cue.Yay_Cue" (`self.K2_GetActorLocation`) (struct) 1.0 1.0 0.0 null null null null)))))

(event `self.SM_Coin.OnComponentBeginOverlap`
  (params (OverlappedComponent :type "PrimitiveComponent Object Reference") (OtherActor :type "Actor Object Reference") (OtherComp :type "PrimitiveComponent Object Reference") (OtherBodyIndex :type Integer) (bFromSweep :type Boolean) (SweepResult :type "HitResult Structure (by ref)"))
  (cast `/Game/ThirdPerson/Blueprints/BP_ThirdPersonCharacter` OtherActor)
  (`NiagaraFunctionLibrary.SpawnSystemAtLocation` "/Game/sA_PickupSet_1/Fx/NiagaraSystems/NS_CoinBurst.NS_CoinBurst" (`SceneComponent.K2_GetComponentLocation` (`self.SM_Coin`))))

(fn `UserConstructionScript`
  (`StaticMeshComponent.SetStaticMesh` (`self.SM_WaterBarrierLight`) (`self.Mesh`)))