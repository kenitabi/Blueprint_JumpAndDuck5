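; BP_Lift is a lift actor that shuttles vertically between its starting height and a top height set by the TopLocation Z offset.
; BeginPlay caches both height limits, and Tick applies MovingLocation as an unswept local offset each frame, so speed depends on frame rate.
; Passing either limit zeroes the offset, then a Delay in Tick pauses the lift before sending it the opposite way.
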(event `self.ReceiveBeginPlay`
  (bind (_returnvalue_x _returnvalue_y _returnvalue_z) (`KismetMathLibrary.BreakVector` (`self.K2_GetActorLocation`)))
  (bind (_toplocation_x _toplocation_y _toplocation_z) (`KismetMathLibrary.BreakVector` (`self.TopLocation`)))
  (set `self.EndLocationZ` (+ _returnvalue_z _toplocation_z))
  (set `self.StartLocationZ` _returnvalue_z))

(event `self.ReceiveTick`
  (params (DeltaSeconds :type "Float (single-precision)"))
  (bind (_returnvalue_x _returnvalue_y _returnvalue_z) (`KismetMathLibrary.BreakVector` (`self.K2_GetActorLocation`)))
  (bind (_returnvalue_x_2 _returnvalue_y_2 _returnvalue_z_2) (`KismetMathLibrary.BreakVector` (`self.K2_GetActorLocation`)))
  (`self.K2_AddActorLocalOffset` (`self.MovingLocation`))
  (if (> _returnvalue_z_2 (`self.EndLocationZ`))
    (set `self.MovingLocation` (0.0 0.0 0.0))
    (`KismetSystemLibrary.Delay` 5.0)
    (set `self.MovingLocation` (0.0 0.0 -20.0))
    (elif (< _returnvalue_z (`self.StartLocationZ`))
      (set `self.MovingLocation` (0.0 0.0 0.0))
      (`KismetSystemLibrary.Delay` 5.0)
      (set `self.MovingLocation` (0.0 0.0 20.0)))))

(fn `UserConstructionScript`)