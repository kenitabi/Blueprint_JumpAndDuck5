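; VFX_Book is an example Blueprint for a skeletal mesh book that tumbles continuously from a random orientation.
; The construction script randomizes the mesh's world rotation and builds LocalRotation from random pitch and yaw, with zero roll, scaled by RotationSpeed.
; Tick adds that rotation locally every frame without delta-time scaling, so the spin rate depends on frame rate.
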(event `self.ReceiveTick`
  (params (DeltaSeconds :type "Float (single-precision)"))
  ;[0 0 0] Add constant rotation
  (`SceneComponent.K2_AddLocalRotation` (`self.SkeletalMesh`) (`self.LocalRotation`) false false))

(fn `UserConstructionScript`
  ;[0 0 0] Set initial random rotation
  (`SceneComponent.K2_SetWorldRotation` (`self.SkeletalMesh`) (`KismetMathLibrary.RandomRotator` true) false false)
  ;[0 0 0] Make random local rotation
  (set `self.LocalRotation` (* (`KismetMathLibrary.MakeRotator` 0.0 (`KismetMathLibrary.ClampAxis` (`KismetMathLibrary.RandomFloatInRange` -1.0 1.0)) (`KismetMathLibrary.ClampAxis` (`KismetMathLibrary.RandomFloatInRange` -1.0 1.0))) (`self.RotationSpeed`))))